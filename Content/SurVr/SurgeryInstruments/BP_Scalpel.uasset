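; BP_Scalpel is a surgical instrument that cuts procedural meshes on BP_Face actors.
; When its reach-distance collision component begins overlapping one of those meshes, BodyCutOff slices it along a plane set by that component's location and right vector.
; The cut creates an uncapped other half with physics off, then teleports both pieces apart along the plane normal to open a gap.
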(event `self.C_ReachDistance.OnComponentBeginOverlap`
  (params (OverlappedComponent :type "PrimitiveComponent Object Reference") (OtherActor :type "Actor Object Reference") (OtherComp :type "PrimitiveComponent Object Reference") (OtherBodyIndex :type Integer) (bFromSweep :type Boolean) (SweepResult :type "HitResult Structure (by ref)"))
  (if (== (`GameplayStatics.GetObjectClass` OtherActor) "/Game/SurVr/Body/BP_Face.BP_Face_C")
    (bind _asprocedural_mesh_component (cast `ProceduralMeshComponent` OtherComp))
    (`self.BodyCutOff` _asprocedural_mesh_component)))

(fn `BodyCutOff`
  (params (CuttedComponent :type "ProceduralMeshComponent Object Reference"))
  (locals (PM_Cutted :type "ProceduralMeshComponent Object Reference"))
  (bind _c_reachdistance (`self.C_ReachDistance`))
  (bind _returnvalue (`SceneComponent.K2_GetComponentLocation` (`local.PM_Cutted`)))
  (bind _returnvalue_2 (* (`SceneComponent.GetRightVector` (`self.C_ReachDistance`)) 20))
  (bind _output_get (set `local.PM_Cutted` CuttedComponent))
  (bind _outotherhalfprocmesh (`KismetProceduralMeshLibrary.SliceProceduralMesh` _output_get (`SceneComponent.K2_GetComponentLocation` _c_reachdistance) (`SceneComponent.GetRightVector` _c_reachdistance) true "NoCap"))
  (`PrimitiveComponent.SetSimulatePhysics` _outotherhalfprocmesh false)
  (`SceneComponent.K2_SetWorldLocation` _outotherhalfprocmesh (- _returnvalue _returnvalue_2) false true)
  (`SceneComponent.K2_SetWorldLocation` (`local.PM_Cutted`) (+ _returnvalue _returnvalue_2) false true)
  (return))

(fn `UserConstructionScript`
  (`parent.UserConstructionScript`))