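; Scalpel surgery instrument that cuts a procedural face mesh in two on contact.
; When ReachDistance begins overlapping, it checks the other component against Face_BP, casts it to ProceduralMeshComponent and calls CutOff.
; CutOff slices the mesh on a plane from ReachDistance's location and right vector, without capping.
; It disables physics on the new half and teleports both halves apart along that vector.
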(event `self.ReachDistance.OnComponentBeginOverlap`
  (params (OverlappedComponent :type "PrimitiveComponent Object Reference") (OtherActor :type "Actor Object Reference") (OtherComp :type "PrimitiveComponent Object Reference") (OtherBodyIndex :type Integer) (bFromSweep :type Boolean) (SweepResult :type "HitResult Structure (by ref)"))
  (if (== (`GameplayStatics.GetObjectClass` OtherComp) "/Game/Body/Body_BP/Face_BP.Face_BP_C")
    (bind _asprocedural_mesh_component (cast `ProceduralMeshComponent` OtherComp))
    (`self.CutOff` _asprocedural_mesh_component)))

(fn `CutOff`
  (params (CuttedComponent :type "ProceduralMeshComponent Object Reference"))
  (locals (CuttedComp :type "ProceduralMeshComponent Object Reference"))
  (bind _reachdistance (`self.ReachDistance`))
  (bind _returnvalue (`SceneComponent.K2_GetComponentLocation` (`local.CuttedComp`)))
  (bind _returnvalue_2 (* (`SceneComponent.GetRightVector` (`self.ReachDistance`)) 20))
  (bind _output_get (set `local.CuttedComp` CuttedComponent))
  (bind _outotherhalfprocmesh (`KismetProceduralMeshLibrary.SliceProceduralMesh` _output_get (`SceneComponent.K2_GetComponentLocation` _reachdistance) (`SceneComponent.GetRightVector` _reachdistance) true "NoCap"))
  (`PrimitiveComponent.SetSimulatePhysics` _outotherhalfprocmesh false)
  (`SceneComponent.K2_SetWorldLocation` _outotherhalfprocmesh (- _returnvalue _returnvalue_2) false true)
  (`SceneComponent.K2_SetWorldLocation` (`local.CuttedComp`) (+ _returnvalue_2 _returnvalue) false true))

(fn `UserConstructionScript`
  (`parent.UserConstructionScript`))